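; BP_redcar is a looping moving car, apparently traffic in a Crossy Road-style game.
; Tick pushes it along local Y by a fixed, unswept offset per frame, so its speed depends on frame rate.
; BeginPlay stores the spawn location, then a Delay loop teleports the car back there every few seconds.
; RestartBeginning and Start duplicate that reset but are uncalled here, and the cleared "StartBegin" timer is never set here.
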(event `self.ReceiveTick`
  (params (DeltaSeconds :type "Float (single-precision)"))
  (`self.K2_AddActorLocalOffset` (0.0 100.0 0.0)))

(event `self.ReceiveBeginPlay`
  (set `self.spawnPoint` (`SceneComponent.K2_GetComponentLocation` (`self.DefaultSceneRoot`)))
  (`KismetSystemLibrary.Delay` 7.0 :!label _label)
  (`KismetSystemLibrary.K2_ClearTimer` null "StartBegin")
  (`self.K2_SetActorLocation` (`self.spawnPoint`))
  (goto _label))

(fn `RestartBeginning`
  (`self.K2_SetActorLocation` (`self.spawnPoint`)))

(fn `Start`
  (`self.K2_SetActorLocation` (`self.spawnPoint`)))

(fn `UserConstructionScript`)