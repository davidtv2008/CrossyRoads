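; BP_Player is the player pawn for CrossyR, moved forward and sideways by axis input scaled by MaxSpeed.
; Each tick it consumes the accumulated input vector and applies it as a swept, frame-rate-independent local offset, without a movement component.
; The camera uses absolute location and rotation, trailing the player on X while Y and height stay fixed.
; BeginPlay applies a one-time local rotation; NotFloor is an empty stub.
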(event `InputAxis|MoveForward`
  (params (AxisValue :type "Float (single-precision)"))
  (`self.AddMovementInput` (`self.GetActorForwardVector`) (* AxisValue (`self.MaxSpeed`))))

(event `self.ReceiveBeginPlay`
  (`self.K2_AddActorLocalRotation` (struct :`Yaw` -90.0))
  (`SceneComponent.SetAbsolute` (`self.Camera`) true true false))

(event `InputAxis|MoveSides`
  (params (AxisValue :type "Float (single-precision)"))
  (`self.AddMovementInput` (`self.GetActorRightVector`) (* AxisValue (`self.MaxSpeed`))))

(event `self.ReceiveTick`
  (params (DeltaSeconds :type "Float (single-precision)"))
  (`SceneComponent.K2_SetWorldLocation` (`self.Camera`) (`KismetMathLibrary.MakeVector` (- (.x (`self.K2_GetActorLocation`)) 500.0) 800.0 1600.0) false false)
  (bind _returnvalue (`self.ConsumeMovementInputVector`))
  (`self.K2_AddActorLocalOffset` (* _returnvalue DeltaSeconds) true))

(fn `notFloor`
  (params (NewParam :type Boolean)))

(fn `UserConstructionScript`)